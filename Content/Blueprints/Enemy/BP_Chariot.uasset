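; BP_Chariot is an enemy chariot built on physics constraints, which drives while a target is in range and can fall apart.
; Each Tick, IsTargetInRange switches angular velocity targets on four axis constraints between spinning, with alternating signs, and zero.
; BreakPhysicsConstraintEvent waits briefly, then breaks all four axis and four suspension constraints to detach those parts.
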(event `self.ReceiveTick`
  (params (DeltaSeconds :type "Float (single-precision)"))
  (bind _pc_axis1 (`self.PC_Axis1`))
  (bind _pc_axis2 (`self.PC_Axis2`))
  (bind _pc_axis3 (`self.PC_Axis3`))
  (bind _pc_axis4 (`self.PC_Axis4`))
  (if (`self.IsTargetInRange`)
    (`PhysicsConstraintComponent.SetAngularVelocityTarget` _pc_axis1 (1.0 0.0 0.0))
    (`PhysicsConstraintComponent.SetAngularVelocityTarget` _pc_axis2 (-1.0 0.0 0.0))
    (`PhysicsConstraintComponent.SetAngularVelocityTarget` _pc_axis3 (1.0 0.0 0.0))
    (`PhysicsConstraintComponent.SetAngularVelocityTarget` _pc_axis4 (-1.0 0.0 0.0))
    (else
      (`PhysicsConstraintComponent.SetAngularVelocityTarget` _pc_axis1 (0.0 0.0 0.0))
      (`PhysicsConstraintComponent.SetAngularVelocityTarget` _pc_axis2 (0.0 0.0 0.0))
      (`PhysicsConstraintComponent.SetAngularVelocityTarget` _pc_axis3 (0.0 0.0 0.0))
      (`PhysicsConstraintComponent.SetAngularVelocityTarget` _pc_axis4 (0.0 0.0 0.0)))))

(event `self.BreakPhysicsConstraintEvent`
  (`KismetSystemLibrary.Delay` 0.15)
  (`PhysicsConstraintComponent.BreakConstraint` (`self.PC_Axis2`))
  (`PhysicsConstraintComponent.BreakConstraint` (`self.PC_Suspension2`))
  (`PhysicsConstraintComponent.BreakConstraint` (`self.PC_Suspension3`))
  (`PhysicsConstraintComponent.BreakConstraint` (`self.PC_Axis3`))
  (`PhysicsConstraintComponent.BreakConstraint` (`self.PC_Suspension4`))
  (`PhysicsConstraintComponent.BreakConstraint` (`self.PC_Axis4`))
  (`PhysicsConstraintComponent.BreakConstraint` (`self.PC_Axis1`))
  (`PhysicsConstraintComponent.BreakConstraint` (`self.PC_Suspension1`)))

(fn `UserConstructionScript`)