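; Player character Blueprint that adds foot-attached force actors, switchable camera views and recovery after leaving a vehicle.
; BeginPlay spawns two BP_Dynamic_Force_Component actors and attaches them to the left and right foot sockets.
; SwitchtoView uses per-view timelines to blend the camera boom socket offset to normal, aiming or grabbing positions.
; After vehicle detach, short delays bracket reactivating CharacterMovement, then the saved location is restored and velocity zeroed.
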(event `self.ReceiveBeginPlay`
  (bind _returnvalue (`self.GetTransform`))
  (bind _returnvalue_2 (`|SpawnActorFromClass` "/Water/FluidSimulation/Blueprints/Examples/BP_Dynamic_Force_Component.BP_Dynamic_Force_Component_C" _returnvalue "Undefined" "MultiplyWithRoot" self null))
  (`self.K2_AttachToComponent` _returnvalue_2 (`self.Mesh`) "LeftFootSocket" "SnapToTarget" "SnapToTarget" "SnapToTarget" true)
  (bind _returnvalue_3 (`|SpawnActorFromClass` "/Water/FluidSimulation/Blueprints/Examples/BP_Dynamic_Force_Component.BP_Dynamic_Force_Component_C" _returnvalue "Undefined" "MultiplyWithRoot" self null))
  (`self.K2_AttachToComponent` _returnvalue_3 (`self.Mesh`) "RightFootSocket" "SnapToTarget" "SnapToTarget" "SnapToTarget" true))

(event `self.SwitchToView`
  (params (NewItTakesXView :type "EItTakesXViewType Enum" :default "EItTakesXViewType_Normal"))
  (bind _originsocketoffset (`self.OriginSocketOffset`))
  (bind _originsocketoffset_2 (`self.OriginSocketOffset`))
  (bind _output_get (set `self.OriginSocketOffset` (`SpringArmComponent.SocketOffset` (`self.CameraBoom`))))
  (switch `EItTakesXViewType` NewItTakesXView
    (:`EItTakesXViewType_Normal`
      (bind (_direction _value) (`Timeline|SwitchNormal` :!via `PlayFromStart`)
        (:`Update`
          (set `SpringArmComponent.SocketOffset` (+ (* (- (`KismetMathLibrary.Vector_Zero`) _originsocketoffset_2) _value) _originsocketoffset_2) (`self.CameraBoom`)))))
    (:`EItTakesXViewType_NiceToAiming`
      (bind (_direction_2 _value_2) (`Timeline|SwitchToNiceToAming` :!via `PlayFromStart`)
        (:`Update`
          (set `SpringArmComponent.SocketOffset` (+ (* (- (`self.CameraSocketOffsetNiceToAiming`) (`self.OriginSocketOffset`)) _value_2) _output_get) (`self.CameraBoom`)))))
    (:`EItTakesXViewType_NiceToGrabbing`
      (bind (_direction_3 _value_3) (`Timeline|SwitchToNiceToGrabbing` :!via `PlayFromStart`)
        (:`Update`
          (set `SpringArmComponent.SocketOffset` (+ (* (- (`self.CameraSocketOffsetNiceToGrab`) _originsocketoffset) _value_3) _originsocketoffset) (`self.CameraBoom`)))))))

(event `self.AfterDetachFromVehicle`
  (bind _charactermovement (`self.CharacterMovement`))
  (bind _output_get (set `self.CharacterLocationAfterActiveMovement` (`self.K2_GetActorLocation`)))
  (`KismetSystemLibrary.Delay` 0.01)
  (`ActorComponent.SetActive` _charactermovement true false)
  (`KismetSystemLibrary.Delay` 0.01)
  (`self.K2_SetActorLocation` _output_get)
  (set `MovementComponent.Velocity` (0.0 0.0 0.0) _charactermovement))

(fn `UserConstructionScript`)