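; One-shot Chaos field actor that breaks destructibles inside its sphere and flings the fragments outward, then destroys itself on BeginPlay.
; A radial falloff with no attenuation, sized and centered on the Sphere component, applies external cluster strain to fracture geometry.
; A radial vector field then applies linear velocity, using a culling field built on the same falloff to cull the effect outside the sphere.
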(event `self.ReceiveBeginPlay`
  (bind _fieldsystemcomponent (`self.FieldSystemComponent`))
  (bind _sphere (`self.Sphere`))
  (bind _returnvalue (`SceneComponent.K2_GetComponentLocation` _sphere))
  (bind _returnvalue_2 (`RadialFalloff.SetRadialFalloff` (`self.RadialFalloff`) (`self.RadialFallOffFieldMagnitude`) 0.0 1.0 0.0 (`SphereComponent.GetScaledSphereRadius` _sphere) _returnvalue "Field_FallOff_None"))
  ;[1 1 1] 添加使chaos破坏的力
  (`FieldSystemComponent.ApplyPhysicsField` _fieldsystemcomponent true "Field_ExternalClusterStrain" null _returnvalue_2)
  ;[1 1 1] 添加使碎块飞溅的速度
  (`FieldSystemComponent.ApplyPhysicsField` _fieldsystemcomponent true "Field_LinearVelocity" null (`CullingField.SetCullingField` (`self.CullingField`) _returnvalue_2 (`RadialVector.SetRadialVector` (`self.RadialVector`) (`self.RadialVectorFieldMagnitude`) _returnvalue) "Field_Culling_Outside"))
  (`self.K2_DestroyActor`))

(fn `UserConstructionScript`)