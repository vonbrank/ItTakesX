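; BP_DamageSphereEmitter is an environment hazard that continuously spawns BP_DamageSphere actors.
; From BeginPlay, a looping Delay chain cycles through three spawn point components in order, waiting EmittingInterval before each spawn.
; Each spawned sphere gets its lifespan set to LifeTime, so it removes itself without cleanup by the emitter.
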(event `self.ReceiveBeginPlay`
  (bind _lifetime (`self.LifeTime`))
  (`KismetSystemLibrary.Delay` (`self.EmittingInterval`) :!label _label)
  (bind _returnvalue (`|SpawnActorFromClass` "/Game/Blueprints/Environment/BP_DamageSphere.BP_DamageSphere_C" (`SceneComponent.K2_GetComponentToWorld` (`self.SpawnPoint1`)) "Undefined" "MultiplyWithRoot" null null))
  (`self.SetLifeSpan` _returnvalue _lifetime)
  (`KismetSystemLibrary.Delay` (`self.EmittingInterval`))
  (bind _returnvalue_2 (`|SpawnActorFromClass` "/Game/Blueprints/Environment/BP_DamageSphere.BP_DamageSphere_C" (`SceneComponent.K2_GetComponentToWorld` (`self.SpawnPoint2`)) "Undefined" "MultiplyWithRoot" null null))
  (`self.SetLifeSpan` _returnvalue_2 _lifetime)
  (`KismetSystemLibrary.Delay` (`self.EmittingInterval`))
  (bind _returnvalue_3 (`|SpawnActorFromClass` "/Game/Blueprints/Environment/BP_DamageSphere.BP_DamageSphere_C" (`SceneComponent.K2_GetComponentToWorld` (`self.SpawnPoint3`)) "Undefined" "MultiplyWithRoot" null null))
  (`self.SetLifeSpan` _returnvalue_3 _lifetime)
  (goto _label))

(fn `UserConstructionScript`)