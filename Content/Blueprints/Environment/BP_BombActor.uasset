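; BP_BombActor is a bomb actor that reverses time after it has exploded and then explodes again.
; HandHasExploded calls TimeReverse, waits CaptureTime plus ExplodeAgainInterval, then calls ExplodeAgain, with both functions defined outside this graph.
; An IsReversing flag ignores repeat triggers until a final CaptureTime delay completes.
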(event `self.HandHasExploded`
  (bind _capturetime (`self.CaptureTime`))
  (if (not (`self.bIsReversing`))
    (set `self.bIsReversing` true)
    (`self.TimeReverse`)
    (`KismetSystemLibrary.Delay` _capturetime)
    (`KismetSystemLibrary.Delay` (`self.ExplodeAgainInterval`))
    (`self.ExplodeAgain`)
    (`KismetSystemLibrary.Delay` _capturetime)
    (set `self.bIsReversing` false)))

(fn `UserConstructionScript`)